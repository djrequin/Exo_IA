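; Quest pedestal that, on interaction, spawns a copy of the player's held item at its sphere's transform.
; It takes the held class from the character, either from ClassInHand or the actor in hand.
; If the spawned actor carries the needed tag, the related NPC's dialogue switches to its quest-finished content.
; A "triche" cheat event forces a purple battery through the same check, then destroys it after a short delay.
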(event Custom|triche
  (bind _related_pnj (Variables|Default|GetRelated_PNJ))
  (Variables|Default|Setclass%20to%20spawn "/Game/Batteries/BP_batterie_Violet.BP_batterie_Violet_C")
  (Utilities|FlowControl|Sequence
    (:then_0
      (bind _returnvalue (Game|SpawnActorfromClass (Variables|Default|Getclass%20to%20spawn) (Transformation|GetWorldTransform (Variables|Default|GetSphere)) "Undefined" "MultiplyWithRoot" 0 0))
      (if (Actor|ActorHasTag _returnvalue (Utilities|String|StringToName (Variables|Default|GetNeeded_Tag)))
        (Variables|/Game/Quest/AI/AI_PNJ.AI_PNJ_C|SetContent2 _related_pnj (Variables|/Game/Quest/AI/AI_PNJ.AI_PNJ_C|GetQuest_finished _related_pnj))
        (else
          (Development|PrintString (Utilities|String|ToString(Boolean) (Actor|ActorHasTag _returnvalue (Utilities|String|StringToName (Variables|Default|GetNeeded_Tag))))))))
    (:then_1
      (Utilities|FlowControl|Delay 0.45)
      (Actor|DestroyActor _returnvalue))))

(event EventInteraction
  (params (Touched_actor :type Actor%20Object%20Reference) (component :type Primitive%20Component%20Object%20Reference) (Actor_in_hand :type Actor%20Object%20Reference))
  (bind _related_pnj (Variables|Default|GetRelated_PNJ))
  (bind _asbp_third_person_character (Utilities|Casting|CastToBP_ThirdPersonCharacter (Game|GetPlayerCharacter 0)))
  ;[0 0 0] J'aurais dû refaire mon système de spawn mais flemme
  (Variables|Default|SetAs%20BP%20Third%20Person%20Character _asbp_third_person_character)
  (if (== (Variables|/Game/ThirdPerson/Blueprints/BP_ThirdPersonCharacter.BP_ThirdPersonCharacter_C|GetClass_in_hand _asbp_third_person_character) 0)
    (Variables|Default|Setclass%20to%20spawn (Utilities|GetClass (Variables|/Game/ThirdPerson/Blueprints/BP_ThirdPersonCharacter.BP_ThirdPersonCharacter_C|GetActor_in_hand (Variables|Default|GetAs%20BP%20Third%20Person%20Character))))
    (else
      (Variables|Default|Setclass%20to%20spawn (Variables|/Game/ThirdPerson/Blueprints/BP_ThirdPersonCharacter.BP_ThirdPersonCharacter_C|GetClass_in_hand _asbp_third_person_character))))
  (bind _returnvalue (Game|SpawnActorfromClass (Variables|Default|Getclass%20to%20spawn) (Transformation|GetWorldTransform (Variables|Default|GetSphere)) "Undefined" "MultiplyWithRoot" 0 0))
  (if (Actor|ActorHasTag _returnvalue (Utilities|String|StringToName (Variables|Default|GetNeeded_Tag)))
    (Variables|/Game/Quest/AI/AI_PNJ.AI_PNJ_C|SetContent2 _related_pnj (Variables|/Game/Quest/AI/AI_PNJ.AI_PNJ_C|GetQuest_finished _related_pnj))
    (else
      (Development|PrintString (Utilities|String|ToString(Boolean) (Actor|ActorHasTag _returnvalue (Utilities|String|StringToName (Variables|Default|GetNeeded_Tag))))))))

(fn ConstructionScript)