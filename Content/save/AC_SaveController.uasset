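; Save controller component that creates, saves, loads and checks the game's Save_Manager save object in a named slot.
; CreateGame builds the object with a placeholder player ID and the slot name, storing it in CurrentSaveDatas for SaveGame to write.
; LoadGame reads the slot back synchronously; its async branch calls AsyncLoadOrCreateSaveGameForLocalPlayer without storing a result.
; DeleteGame is an empty stub.
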(event EventBeginPlay)

(event EventTick
  (params (DeltaSeconds :type Float%20%28single-precision%29)))

(fn SaveGame
  (SaveGame|SaveGametoSlot (Variables|Default|GetCurrent%20save%20datas) (Variables|Default|GetSlot%20Name)))

(fn LoadGame
  (params (Async :type Boolean))
  (if Async
    (Class|LocalPlayerSaveGame|AsyncLoadorCreateSaveGameforLocalPlayer)
    (else
      (bind _returnvalue (SaveGame|LoadGamefromSlot (Variables|Default|GetSlot%20Name)))
      (bind _assave_manager (Utilities|Casting|CastToSave_Manager _returnvalue))
      (Variables|Default|SetCurrent%20save%20datas _assave_manager))))

(fn CreateGame
  (bind _returnvalue (SaveGame|CreateSaveGameObject "/Game/save/Save_Manager.Save_Manager_C"))
  (bind _output_get (Variables|Default|SetCurrent%20save%20datas _returnvalue))
  ;[1 1 1] adapter l'ID à celui du profil du joueur
  (Variables|/Game/save/Save_Manager.Save_Manager_C|SetPlayer%20ID _output_get 0)
  ;[1 1 1] default value
  (Variables|/Game/save/Save_Manager.Save_Manager_C|SetSaveSlotName _output_get (Variables|Default|GetSlot%20Name)))

(fn DeleteGame)

(fn CheckSave
  (bind _returnvalue (SaveGame|DoesSaveGameExist (Variables|Default|GetSlot%20Name)))
  (return _returnvalue))