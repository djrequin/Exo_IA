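; Parent Blueprint for battery actors that the player can pick up through an Interaction event.
; Interaction passes the battery to the third-person character's PutObjectInHand.
; Any valid object returned moves to the battery's world transform, effectively swapping places.
; The battery's root then has SetWorldTransform called with no transform supplied, and a debug string prints.
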(event EventBeginPlay)

(event Collision|EventActorBeginOverlap
  (params (OtherActor :type Actor%20Object%20Reference)))

(event EventTick
  (params (DeltaSeconds :type Float%20%28single-precision%29)))

(event EventInteraction
  (params (Touched_actor :type Actor%20Object%20Reference) (component :type Primitive%20Component%20Object%20Reference))
  (bind _asbp_third_person_character (Utilities|Casting|CastToBP_ThirdPersonCharacter (Game|GetPlayerCharacter 0)))
  (bind _previous_actor (Default|PutObjectinHand _asbp_third_person_character self))
  (Utilities|IsValid _previous_actor
    (:Is%20Valid
      (Transformation|SetActorTransform _previous_actor (Transformation|GetWorldTransform (Variables|Default|GetDefaultSceneRoot))))
    (:Is%20Not%20Valid
      _))
  (Transformation|SetWorldTransform (Variables|Default|GetDefaultSceneRoot) (Math|Transform|MakeTransform "0, 0, 0" "0, 0, 0" "1.000000,1.000000,1.000000") false false)
  (Development|PrintString "Hello"))

(fn ConstructionScript)