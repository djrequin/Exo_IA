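; Goblin enemy Blueprint that registers itself with its AIC_Goblin controller on BeginPlay.
; PawnSensing passes the distance to seen "detectable_ennemy" pawns to the controller, which checks it and forwards the results through WarnBBDistance.
; Two box overlaps, gated by the controller's first and second attack flags, only print hit debug text without applying damage.
; A TraceLine helper, not called here, returns a debug-drawn box trace's impact point.
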(event OnSeePawn(PawnSensing)
  (params (Pawn :type Pawn%20Object%20Reference))
  (bind _aic_goblin (Variables|Default|GetAIC%20Goblin))
  ;[1 1 1] Détection du joueur et calcul de la distance avec ce dernier
  (if (Actor|ActorHasTag Pawn "detectable_ennemy")
    (bind _output_get (Variables|Default|SetSeen_Pawn Pawn))
    (bind (__15 __10) (Default|CheckDistance _aic_goblin (Transformation|GetDistanceTo _output_get self)))
    (Default|WarnBBDistance _aic_goblin __10 __15)))

(event OnComponentBeginOverlap(Box)
  (params (OverlappedComponent :type Primitive%20Component%20Object%20Reference) (OtherActor :type Actor%20Object%20Reference) (OtherComp :type Primitive%20Component%20Object%20Reference) (OtherBodyIndex :type Integer) (bFromSweep :type Boolean) (SweepResult :type Hit%20Result%20Structure%20%28by%20ref%29))
  ;[1 1 1] DGts attaque 1
  (if (Variables|/Game/AI_Gob/AIC_Goblin.AIC_Goblin_C|GetIn_1st_atk (Variables|Default|GetAIC%20Goblin))
    (if (Actor|ActorHasTag OtherActor "detectable_ennemy")
      (Development|PrintString "hit")
      (else
        (Development|PrintString "nop")))))

(event OnComponentBeginOverlap(Box1)
  (params (OverlappedComponent :type Primitive%20Component%20Object%20Reference) (OtherActor :type Actor%20Object%20Reference) (OtherComp :type Primitive%20Component%20Object%20Reference) (OtherBodyIndex :type Integer) (bFromSweep :type Boolean) (SweepResult :type Hit%20Result%20Structure%20%28by%20ref%29))
  ;[1 1 1] Dgts attaque 2
  (if (Variables|/Game/AI_Gob/AIC_Goblin.AIC_Goblin_C|GetIn_2nd_atk (Variables|Default|GetAIC%20Goblin))
    (if (Actor|ActorHasTag OtherActor "detectable_ennemy")
      (Development|PrintString "hit")
      (else
        (Development|PrintString "nop")))))

(event EventBeginPlay
  (bind _asaic_goblin (Utilities|Casting|CastToAIC_Goblin (AI|GetAIController self)))
  (bind _output_get (Variables|Default|SetAIC%20Goblin _asaic_goblin))
  (Variables|/Game/AI_Gob/AIC_Goblin.AIC_Goblin_C|SetControlled_Enemy _output_get self))

(fn ConstructionScript)

(fn TraceLine
  (bind _self self)
  (bind _returnvalue (Transformation|GetActorLocation _self))
  (bind _outhit (Collision|BoxTraceByChannel _returnvalue (- (* _returnvalue (Transformation|GetActorForwardVector)) 2e+03) (Math|Vector|MakeVector 2e+01 2e+01 3e+01) "0, 0, 0" "TraceTypeQuery1" false 0 "Persistent"))
  (return (.ImpactPoint (Collision|BreakHitResult _outhit))))